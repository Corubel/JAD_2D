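; BP_enemy_base is a base enemy for a side-scroller that moves horizontally and damages the player on contact.
; Its custom Direction event uses EnemyMoveRight to yaw the sprite and add movement input along the X axis; nothing in this file calls it.
; A capsule hit on a 2DSideScrollerCharacter stores that character as PlayerRef and applies damage to it.
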(event `Direction`
  (`SceneComponent.K2_SetRelativeRotation` (`self.Sprite`) (`KismetMathLibrary.MakeRotator` 0.0 0.0 (`KismetMathLibrary.SelectFloat` 0.0 180.0 (`self.enemyMoveRight`))) false false)
  (`self.AddMovementInput` (`KismetMathLibrary.SelectVector` (1.0 0.0 0.0) (-1.0 0.0 0.0) (`self.enemyMoveRight`))))

(event `self.CapsuleComponent.OnComponentHit`
  (params (HitComponent :type "PrimitiveComponent Object Reference") (OtherActor :type "Actor Object Reference") (OtherComp :type "PrimitiveComponent Object Reference") (NormalImpulse :type "Vector Structure") (Hit :type "HitResult Structure (by ref)"))
  (bind _as2dside_scroller_character (cast `/Game/MyProyect/Character/2DSideScrollerCharacter` OtherActor))
  (set `self.player_ref` _as2dside_scroller_character)
  (`GameplayStatics.ApplyDamage` (`self.player_ref`) 1.0))

(fn `UserConstructionScript`)